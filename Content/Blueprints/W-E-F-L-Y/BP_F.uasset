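; BP_F is a letter pickup, likely one of a set, that the first-person character collects by overlapping it.
; On overlap it loops over the actor's Tags, plays a pickup sound, destroys itself and appends each tag's text to LettersAcquired on BP_PlayerController.
; The letter value comes from the actor tags rather than a dedicated variable.
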(event Collision|EventActorBeginOverlap
  (params (OtherActor :type Actor%20Object%20Reference))
  (Utilities|Casting|CastToBP_FirstPersonCharacter OtherActor)
  (for _array_element (Variables|Actor|GetTags)
    (bind _asbp_player_controller (Utilities|Casting|CastToBP_PlayerController (Game|GetPlayerController 0)))
    (Audio|PlaySoundatLocation "/Game/Sounds/S_LetterPickUp.S_LetterPickUp" (Transformation|GetActorLocation))
    (Actor|DestroyActor)
    (Variables|/Game/Blueprints/BP_PlayerController.BP_PlayerController_C|SetLettersAcquired _asbp_player_controller (Utilities|String|Append (Variables|/Game/Blueprints/BP_PlayerController.BP_PlayerController_C|GetLettersAcquired _asbp_player_controller) (Utilities|String|ToString(Name) _array_element)))))

(fn ConstructionScript)