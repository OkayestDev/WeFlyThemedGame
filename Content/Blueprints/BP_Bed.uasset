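; BP_Bed is an AI-controlled bed that moves toward the player whenever it has line of sight to them.
; A looping timer started on BeginPlay periodically line traces from the bed to the player's pawn.
; When the trace hits BP_FirstPersonCharacter, the AI controller moves the bed straight to the player's current location without pathfinding.
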(event EventBeginPlay
  (Utilities|Time|SetTimerbyFunctionName 0 "MoveIfPlayerIsVisible" 0.3 true))

(fn ConstructionScript)

(fn MoveifPlayerIsVisible
  (bind _returnvalue (Game|GetPlayerController 0))
  (bind _returnvalue_2 (Pawn|GetControlledPawn _returnvalue))
  (bind _returnvalue_3 (Transformation|GetActorLocation _returnvalue_2))
  (bind _outhit (Collision|LineTraceByChannel (Transformation|GetActorLocation) _returnvalue_3 "TraceTypeQuery3" false 0 "None"))
  (Utilities|Casting|CastToBP_FirstPersonCharacter (.HitActor (Collision|BreakHitResult _outhit)))
  (AI|Navigation|MovetoLocation (AI|GetAIController self) _returnvalue_3 -1.0 true false false))